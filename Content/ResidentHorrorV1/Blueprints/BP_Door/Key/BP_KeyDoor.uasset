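; BP_KeyDoor is a key item that the player picks up and uses to open doors.
; Interacting with it sends the item to the player's inventory.
; Using it runs the parent use logic, then asks the player character's interact component to open a door, passing the item's interact data asset.
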(event EventInteractItem
  (params (ACTO :type Actor%20Object%20Reference) (Player :type BP%20Resident%20Horror%20V1%20Object%20Reference))
  ;[0 0 0] Add item In Inventory
  (CallFunction|SendItemtoInventory Player Player))

(fn ConstructionScript
  (|CallParentFunction))

(fn UseItem
  (bind _sucess (|CallParentFunction))
  (Default|OpenDoor (Variables|/Game/ResidentHorrorV1/Character/BP_Character/BP_Resident_HorrorV1.BP_Resident_HorrorV1_C|GetBPC_Interact (CallFunction|MyCharacterResidentHorror)) (Utilities|Struct|BreakS_Item_Structure (Utilities|Struct|BreakS_SlotStruct (Variables|Default|GetS%20ItemStrucuture))))
  (return _sucess))