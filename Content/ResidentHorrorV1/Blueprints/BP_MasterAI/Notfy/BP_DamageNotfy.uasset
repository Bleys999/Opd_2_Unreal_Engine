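; BP_DamageNotfy is an animation notify state that applies melee-style damage to the Resident Horror player character during an animation window.
; Each tick it sphere-traces for Pawns between two configurable bone sockets on the animated mesh.
; When the hit is the player, it calls TakeDamage on their HealthComponent with a configurable value.
; A HitActors list, cleared at notify begin, guards against repeat damage within one window.
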(fn ReceivedNotifyTick
  (params (MeshComp :type Skeletal%20Mesh%20Component%20Object%20Reference) (Animation :type Anim%20Sequence%20Base%20Object%20Reference) (FrameDeltaTime :type Float%20%28single-precision%29) (EventReference :type Anim%20Notify%20Event%20Reference%20Structure%20%28by%20ref%29))
  (bind (_outhit _returnvalue) (Collision|SphereTraceForObjects MeshComp (Transformation|GetSocketLocation MeshComp (Variables|Configuration|GetStart%20Bone)) (Transformation|GetSocketLocation MeshComp (Variables|Configuration|GetEnd%20Bone)) (Variables|Configuration|GetTrace%20Size) (Utilities|Array|MakeArray "ObjectTypeQuery3") false 0 "None" true "(R=1.000000,G=0.000000,B=0.000000,A=1.000000)" "(R=0.000000,G=1.000000,B=0.000000,A=1.000000)" 0.1))
  (if _returnvalue
    (if (== (.HitActor (Collision|BreakHitResult _outhit)) (CallFunction|MyCharacterResidentHorror MeshComp))
      (LocalVariables|SetHitResult _outhit)
      (Utilities|FlowControl|Sequence
        (:then_0
          (if (not (Utilities|Array|ContainsItem (Variables|Default|GetHitActors) 0))
            (Utilities|Array|Add (Variables|Default|GetHitActors) 0)
            (Utilities|IsValid (.HitActor (Collision|BreakHitResult _outhit))
              (:Is%20Valid
                (Default|TakeDamage (Variables|/Game/ResidentHorrorV1/Character/BP_Character/BP_Resident_HorrorV1.BP_Resident_HorrorV1_C|GetHealthComponent (CallFunction|MyCharacterResidentHorror MeshComp)) (Variables|Configuration|GetDamage%20Value))
                (return false)))))
        (:then_1
          (return false))))))

(fn ReceivedNotifyBegin
  (params (MeshComp :type Skeletal%20Mesh%20Component%20Object%20Reference) (Animation :type Anim%20Sequence%20Base%20Object%20Reference) (TotalDuration :type Float%20%28single-precision%29) (EventReference :type Anim%20Notify%20Event%20Reference%20Structure%20%28by%20ref%29))
  (Utilities|Array|Clear (Variables|Default|GetHitActors))
  (return false))