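; BP_StoredContainer is a container item that shows the player's stored inventory, likely a storage box in a survival-horror game.
; Construction sets the container component's slot count from its StoredSlots value.
; The GetStoredInventory event copies each entry of the player character's StoredInventory into the container's inventory at the same index, while BeginPlay only calls the parent.
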(event EventBeginPlay
  ;[0.15 0.15 0.15 0.5] Not Remove
  (|CallParentFunction))

(event EventGetStoredInventory
  ;[0.15 0.15 0.15 0.5] Get Stored Inventory
  (for (_array_element _array_index) (Variables|/Game/ResidentHorrorV1/Blueprints/BP_Inventory/BPC_Inventory.BPC_Inventory_C|GetStoredInventory (Variables|/Game/ResidentHorrorV1/Character/BP_Character/BP_Resident_HorrorV1.BP_Resident_HorrorV1_C|GetBPC_Inventory (CallFunction|MyCharacterResidentHorror)))
    (Utilities|Array|SetArrayElem (Variables|/Game/ResidentHorrorV1/Blueprints/BP_Inventory/BPC_Inventory.BPC_Inventory_C|GetInventory (Variables|Default|GetBPC_InventoryContainer)) _array_index _array_element)))

(fn ConstructionScript
  (bind _bpc_inventorycontainer (Variables|Default|GetBPC_InventoryContainer))
  (|CallParentFunction)
  (Variables|/Game/ResidentHorrorV1/Blueprints/BP_Inventory/BPC_Inventory.BPC_Inventory_C|SetNumberOfSlots _bpc_inventorycontainer (Variables|/Game/ResidentHorrorV1/Blueprints/BP_Inventory/BPC_Inventory.BPC_Inventory_C|GetStoredSlots _bpc_inventorycontainer)))