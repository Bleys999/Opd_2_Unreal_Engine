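; Interactable save point actor that opens the in-game save menu from a cinematic camera view.
; InteractItem fades out, disables player input, hides the character, creates WBP_SaveIngame with a self reference, switches to the CineCamera and plays save-screen music while lowering the music manager's volume.
; CloseCamera reverses this behind another fade, restoring the pawn view, input and ambient music.
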(event Custom|Initial%20Camera
  ;[0 0 0] have a camera
  (Game|Player|SetViewTargetwithBlend (Game|GetPlayerController 0) (Components|GetOwner (Variables|Default|GetCineCamera)) 0.0 "VTBlend_Cubic" 1.0 false))

(event Custom|Close%20Camera
  (bind _asbp_player (CallFunction|MyCharacterResidentHorror))
  (bind _music_manage_ref (Variables|/Game/ResidentHorrorV1/Character/BP_Character/BP_Resident_HorrorV1.BP_Resident_HorrorV1_C|GetMusic%20manage%20ref _asbp_player))
  (bind _ambiente_sound_component (Variables|/Game/ResidentHorrorV1/Blueprints/BP_MusicAmbient/BP_MusicManager.BP_MusicManager_C|GetAmbiente%20sound%20component _music_manage_ref))
  (bind _sound (Variables|/Script/Engine.AudioComponent|GetSound _ambiente_sound_component))
  ;[0 0 0] Close Camera
  (CameraFades|StartCameraFade :self (Game|GetPlayerCameraManager 0) :ToAlpha 1.0 :Duration 0.3 :bHoldWhenFinished true)
  (Utilities|FlowControl|Delay 0.4)
  (Game|Player|SetViewTargetwithBlend (Game|GetPlayerController 0) (Game|Player|GetPlayerPawn 0) 0.0 "VTBlend_Cubic" 0.0 false)
  (Rendering|SetActorHiddenInGame (CallFunction|MyCharacterResidentHorror) false)
  (Rendering|SetVisibility (Variables|Default|GetWb%20Interact) true false)
  (CameraFades|StartCameraFade :self (Game|GetPlayerCameraManager 0) :FromAlpha 1.0 :Duration 0.4)
  (Input|EnableInput (Game|Player|GetPlayerPawn 0) (Game|GetPlayerController 0))
  (Variables|/Game/ResidentHorrorV1/Character/BP_Character/BP_Resident_HorrorV1.BP_Resident_HorrorV1_C|SetDisable%20camera%20shake? (CallFunction|MyCharacterResidentHorror) false)
  (Audio|Components|Audio|SetSound (Variables|/Game/ResidentHorrorV1/Blueprints/BP_MusicAmbient/BP_MusicManager.BP_MusicManager_C|GetAmbiente%20sound%20component _music_manage_ref) _sound)
  (Default|StartMusicAmbient _music_manage_ref _sound 1.0 1.0)
  (Audio|Components|Audio|Stop (Variables|Default|GetMusic%20Play%20Loading))
  (Variables|/Game/ResidentHorrorV1/Blueprints/BP_MusicAmbient/BP_MusicManager.BP_MusicManager_C|SetReduce%20volume? _music_manage_ref false))

(event EventInteractItem
  (params (ACTO :type Actor%20Object%20Reference) (Player :type BP%20Resident%20Horror%20V1%20Object%20Reference))
  (bind _returnvalue (Game|GetPlayerController 0))
  ;[0 0 0] Interact
  (CameraFades|StartCameraFade :self (Game|GetPlayerCameraManager 0) :ToAlpha 1.0 :Duration 0.3 :bHoldWhenFinished true)
  (Variables|/Game/ResidentHorrorV1/Character/BP_Character/BP_Resident_HorrorV1.BP_Resident_HorrorV1_C|SetDisable%20camera%20shake? (CallFunction|MyCharacterResidentHorror) true)
  (Input|DisableInput (Game|Player|GetPlayerPawn 0) (Game|GetPlayerController 0))
  (Utilities|FlowControl|Delay 0.4)
  (bind _returnvalue_2 (UserInterface|CreateWidget "/Game/ResidentHorrorV1/Blueprints/BP_SaveLoad/WBP_SaveIngame.WBP_SaveIngame_C" 0 self))
  (Variables|Default|SetWB%20SaveInGame _returnvalue_2)
  (UserInterface|Viewport|AddtoViewport _returnvalue_2 0)
  (Variables|/Script/Engine.PlayerController|SetbShowMouseCursor _returnvalue true)
  (Input|SetInputModeUIOnly _returnvalue _returnvalue_2 "DoNotLock" false)
  (CallFunction|InitialCamera)
  (Rendering|SetVisibility (Variables|Default|GetWb%20Interact) false false)
  (Rendering|SetActorHiddenInGame (CallFunction|MyCharacterResidentHorror) true)
  (CameraFades|StartCameraFade :self (Game|GetPlayerCameraManager 0) :FromAlpha 1.0 :Duration 1.0)
  (bind _returnvalue_3 (Actor|GetActorOfClass "/Game/ResidentHorrorV1/Blueprints/BP_MusicAmbient/BP_MusicManager.BP_MusicManager_C"))
  (bind _output_get (Variables|Default|SetBP%20Music%20Manager _returnvalue_3))
  (bind _returnvalue_4 (Audio|SpawnSound2D (Variables|Default|GetMusic%20Play%20Loading%20Screen) 1.0 1.0 0.0 0))
  (Variables|Default|SetMusic%20Play%20Loading _returnvalue_4)
  (Variables|/Game/ResidentHorrorV1/Blueprints/BP_MusicAmbient/BP_MusicManager.BP_MusicManager_C|SetReduce%20volume? _output_get true))

(fn ConstructionScript)